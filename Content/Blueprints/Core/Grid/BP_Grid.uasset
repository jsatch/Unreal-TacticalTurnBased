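; BP_Grid is a grid actor that configures its tile shape, size, count and center in the construction script.
; SpawnGrid stores those parameters, then applies the shape's flat mesh and border material to an InstancedStaticMesh, without adding instances yet.
; GetCurrentShapeData looks up DT_GridShapeData by the shape enum's name, printing an error if missing.
; SpawnGrid also derives the bottom-left corner from center, tile count and tile size.
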(event EventBeginPlay)

(event Collision|EventActorBeginOverlap
  (params (OtherActor :type Actor%20Object%20Reference)))

(event EventTick
  (params (DeltaSeconds :type Float%20%28single-precision%29)))

(fn ConstructionScript
  (CallFunction|SpawnGrid (Variables|Default|GetGridCenterLocation) (Variables|Default|GetGridTileSize) (Variables|Default|GetGridTileCount) (Variables|Default|GetGridShape)))

(fn SpawnGrid
  (params (CenterLocation :type Vector) (TileSize :type Vector) (TileCount :type Vector%202D%20Structure) (Shape :type E_GridShape%20Enum :default "NewEnumerator0"))
  (bind _returnvalue (CallFunction|GetCurrentShapeData))
  (bind _instancedstaticmesh (Variables|Default|GetInstancedStaticMesh))
  (bind (_meshsize _mesh _meshmaterial _flatmesh _flatbordermaterial) (Utilities|Struct|BreakS_GridShapeData _returnvalue))
  (Variables|Default|SetGridCenterLocation CenterLocation)
  (Variables|Default|SetGridTileSize TileSize)
  (Variables|Default|SetGridTileCount TileCount)
  (Variables|Default|SetGridShape Shape)
  (Components|StaticMesh|SetStaticMesh _instancedstaticmesh _flatmesh)
  (Rendering|Material|SetMaterial _instancedstaticmesh 0 _flatbordermaterial)
  (Variables|Default|SetGridBottomLeftCornerLocation (- (Variables|Default|GetGridCenterLocation) (Math|Conversions|ToVector(Vector2D) (* (/ (Variables|Default|GetGridTileCount) 2.0) (Math|Conversions|ToVector2D(Vector) (Variables|Default|GetGridTileSize)))))))

(fn GetCurrentShapeData
  (bind _gridshape (Variables|Default|GetGridShape))
  (bind _returnvalue (Utilities|String|EnumtoString _gridshape))
  (bind _returnvalue_2 (Utilities|GetDataTableRow "/Game/Blueprints/Core/Grid/GridShapes/DT_GridShapeData.DT_GridShapeData" (Utilities|String|StringToName _returnvalue))
    (:then
      _)
    (:RowNotFound
      (Development|PrintString (Utilities|String|Append "ERROR - Enum not found: " _returnvalue) true true "(R=1.000000,G=0.000000,B=0.000000,A=1.000000)" 5.0)))
  (return _returnvalue_2))